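; BP_Brocky is a character Blueprint that adds the WBP_BookieUI widget at BeginPlay and prints jump, organ, limb and appendage counts every Tick.
; Setters for jump velocity, gravity scale, walk speeds and air control store values in Designer variables and print them, without applying them to movement here.
; SetJumpMaxCount writes JumpMaxCount directly.
; SetCurrentHealthPercent does nothing, as its logic is disconnected.
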(event EventBeginPlay
  (bind _returnvalue (UserInterface|CreateWidget "/Game/Blueprints/WBP_BookieUI.WBP_BookieUI_C"))
  (UserInterface|Viewport|AddtoViewport _returnvalue 0))

(event Collision|EventActorBeginOverlap
  (params (OtherActor :type Actor%20Object%20Reference)))

(event EventTick
  (params (DeltaSeconds :type Float%20%28single-precision%29))
  (Development|PrintString (Utilities|String|ToString(Integer) (Variables|Default|GetJumpMaxCount)) true true "(R=0.000000,G=0.660000,B=1.000000,A=1.000000)" 2.0 "Jump Count")
  (Development|PrintString (Utilities|String|ToString(Integer) (Variables|Default|GetNumOrgans)) true true "(R=0.000000,G=0.660000,B=1.000000,A=1.000000)" 2.0 "Num Organs")
  (Development|PrintString (Utilities|String|ToString(Integer) (Variables|Default|GetNumLimbs)) true true "(R=0.000000,G=0.660000,B=1.000000,A=1.000000)" 2.0 "Num Limbs")
  (Development|PrintString (Utilities|String|ToString(Integer) (Variables|Default|GetNumAppendages)) true true "(R=0.000000,G=0.660000,B=1.000000,A=1.000000)" 2.0 "Num Appendages"))

(fn ConstructionScript)

(fn SetJumpMaxCount
  (params (NewJumpMaxCount :type Integer))
  (Development|PrintString "Jumps increased!")
  (Variables|Default|SetJumpMaxCount NewJumpMaxCount))

(fn SetJumpZVelocity
  (params (NewJumpZVelocity :type Integer))
  (Variables|Default|SetDesignerJumpZVelocity (Math|Conversions|ToFloat(Integer) NewJumpZVelocity))
  (Development|PrintString (Utilities|String|Append (Variables|Default|GetVelocity%20Increased) (Utilities|String|ToString(Float) (Variables|Default|GetDesignerJumpZVelocity))) true true "(R=0.000000,G=0.660000,B=1.000000,A=1.000000)" 2.0 "Changed Velocity!"))

(fn SetGravityScale
  (params (NewDesignerGravityScale :type Integer))
  (Variables|Default|SetDesignerGravityScale (Math|Conversions|ToFloat(Integer) NewDesignerGravityScale))
  (Development|PrintString (Utilities|String|Append (Variables|Default|GetGravity%20Scale%20Increased) (Utilities|String|ToString(Float) (Variables|Default|GetDesignerGravityScale))) true true "(R=0.000000,G=0.660000,B=1.000000,A=1.000000)" 2.0 "Gravity Speed"))

(fn SetMaxWalkSpeedCrouched
  (params (MaxWalkSpeedCrouched :type Integer))
  (Variables|Default|SetDesignerMaxWalkSpeedCrouched (Math|Conversions|ToFloat(Integer) MaxWalkSpeedCrouched))
  (Development|PrintString (Utilities|String|Append (Variables|Default|GetMax%20Walk%20Speed%20%28Crouched%29%20Increased) (Utilities|String|ToString(Float) (Variables|Default|GetDesignerMaxWalkSpeedCrouched))) true true "(R=0.000000,G=0.660000,B=1.000000,A=1.000000)" 2.0 "MaxWalkSpeedCrouched"))

(fn SetMaxWalkSpeed
  (params (NewMaxWalkSpeed :type Integer))
  (Variables|Default|SetDesignerMaxWalkSpeed (Math|Conversions|ToFloat(Integer) NewMaxWalkSpeed))
  (Development|PrintString (Utilities|String|Append (Variables|Default|GetMax%20Walk%20Speed%20Increased) (Utilities|String|ToString(Float) (Variables|Default|GetDesignerMaxWalkSpeed))) true true "(R=0.000000,G=0.660000,B=1.000000,A=1.000000)" 2.0 "MaxWalkSpeed"))

(fn SetAirControl
  (params (NewAirControl :type Integer))
  (Variables|Default|SetDesignerAirControl (Math|Conversions|ToFloat(Integer) NewAirControl))
  (Development|PrintString (Utilities|String|Append (Variables|Default|GetAir%20Control%20Increased) (Utilities|String|ToString(Float) (Variables|Default|GetDesignerAirControl))) true true "(R=0.000000,G=0.660000,B=1.000000,A=1.000000)" 2.0 "AirControl"))

(fn SetCurrentHealthPercent
  (params (NewCurrentHealthPercent :type Float%20%28double-precision%29)))